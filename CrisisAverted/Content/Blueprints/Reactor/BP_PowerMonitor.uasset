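; BP_PowerMonitor is a display for the reactor minigame that shows current power and demand as percentage text.
; On entering the minigame it binds to the reactor's power change event and sets both readouts from the minigame's start power.
; Later changes update the power text and recolor it good or bad by status, with low and high both shown as bad; demand stays at its initial value.
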(event `self.MinigameListener.OnEnterMinigame`
  (params (Minigame :type "Minigame Object Reference"))
  (bind _asbp_reactor_minigame (cast `/Game/Blueprints/Minigames/BP_ReactorMinigame` Minigame))
  (add `UnstableOutputBlock.OnChanged` (`/Game/Blueprints/Minigames/BP_ReactorMinigame.Power` _asbp_reactor_minigame) (delegate `OnPowerChanged`))
  (bind _startpower (`/Game/Blueprints/Minigames/BP_ReactorDataAsset.StartPower` (`/Game/Blueprints/Minigames/BP_ReactorMinigame.MinigameData` _asbp_reactor_minigame)))
  (`self.SetDemandDisplay` _startpower)
  (`self.SetPowerDisplay` _startpower "Good"))

(event `OnPowerChanged`
  (params (Value :type "Float (single-precision)") (Status :type "EUnstableMinigameStatus Enum" :default "Low"))
  (`self.SetPowerDisplay` Value Status))

(event `SetPowerDisplay`
  (params (Value :type "Float (single-precision)") (State :type "EUnstableMinigameStatus Enum" :default "Low"))
  (bind _badcolor (`self.BadColor`))
  (bind _powertext (`self.PowerText`))
  (`TextRenderComponent.K2_SetText` _powertext (`|FormatText` "Power: {VAL}" (`KismetTextLibrary.AsPercent_Float` Value "HalfToEven" false true 1 324 0 0)))
  (`TextRenderComponent.SetTextRenderColor` _powertext (select `EUnstableMinigameStatus` State :`Low` _badcolor :`Good` (`self.GoodColor`) :`High` _badcolor)))

(event `SetDemandDisplay`
  (params (Value :type "Float (single-precision)"))
  (`TextRenderComponent.K2_SetText` (`self.DemandText`) (`|FormatText` "Demand: {VAL}" (`KismetTextLibrary.AsPercent_Float` Value "HalfToEven" false true 1 324 0 0))))

(fn `UserConstructionScript`)