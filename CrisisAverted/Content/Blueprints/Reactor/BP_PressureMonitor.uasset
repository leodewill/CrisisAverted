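; BP_PressureMonitor is a text display that shows the reactor minigame's pressure.
; When the minigame listener reports entry, it caches the initial target as base pressure and binds to the Pressure block's value, target and status events.
; The readout shows percentages against that fixed base, offsetting the value by its deviation from the current target, so target changes appear as pressure shifts.
; Status changes recolor the text as good or bad.
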(event `self.MinigameListener.OnEnterMinigame`
  (params (Minigame :type "Minigame Object Reference"))
  (bind _asbp_reactor_minigame (cast `/Game/Blueprints/Minigames/BP_ReactorMinigame` Minigame))
  (`|ExecutionSequence`
    (:`then_0`
      (bind _output_get (set `self.BasePressure` (`/Game/Blueprints/Minigames/BP_ReactorDataAsset.TargetPressure` (`/Game/Blueprints/Minigames/BP_ReactorMinigame.MinigameData` _asbp_reactor_minigame))))
      (`self.OnPressureChanged` _output_get _output_get)
      (`self.OnStatusChanged` "Good" "Good"))
    (:`then_1`
      (`self.BindPressureListeners` (`/Game/Blueprints/Minigames/BP_ReactorMinigame.Pressure` _asbp_reactor_minigame)))))

(event `BindPressureListeners`
  (params (PressureBlock :type "UnstableOutputBlock Object Reference"))
  (`|ExecutionSequence`
    (:`then_0`
      (add `UnstableOutputBlock.OnValueChanged` PressureBlock (delegate `OnPressureChanged`)))
    (:`then_1`
      (add `UnstableOutputBlock.OnTargetChanged` PressureBlock (delegate `OnTargetPressureChanged`)))
    (:`then_2`
      (add `UnstableOutputBlock.OnStatusChanged` PressureBlock (delegate `OnStatusChanged`)))))

(event `OnPressureChanged`
  (params (Value :type "Float (single-precision)") (TargetValue :type "Float (single-precision)"))
  (bind _output_get (set `self.Pressure` Value))
  (`self.SetPressureText` _output_get TargetValue))

(event `SetPressureText`
  (params (Value :type "Float (single-precision)") (TargetValue :type "Float (single-precision)"))
  (`TextRenderComponent.K2_SetText` (`self.PressureText`) (`|FormatText` "Pressure: {VAL} / {BASE}" (`KismetTextLibrary.AsPercent_Float` (+ (- Value TargetValue) (`self.BasePressure`)) "HalfToEven" false true 1 324 0 0) (`KismetTextLibrary.AsPercent_Float` (`self.BasePressure`) "HalfToEven" false true 1 324 0 0))))

(event `OnTargetPressureChanged`
  (params (Value :type "Float (single-precision)"))
  (`self.SetPressureText` (`self.Pressure`) Value))

(event `OnStatusChanged`
  (params (Status :type "EUnstableMinigameStatus Enum" :default "Low") (OldStatus :type "EUnstableMinigameStatus Enum" :default "Low"))
  (bind _badcolor (`self.BadColor`))
  (`TextRenderComponent.SetTextRenderColor` (`self.PressureText`) (select `EUnstableMinigameStatus` Status :`Low` _badcolor :`Good` (`self.GoodColor`) :`High` _badcolor)))

(fn `UserConstructionScript`)