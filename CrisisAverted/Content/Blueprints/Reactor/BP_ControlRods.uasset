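; Control rod lever station for the reactor minigame, letting a player set the reactor's rods.
; Interacting blends the view to the station's camera and leaving blends back to the pawn.
; A slider component drives it: input tilts the lever mesh, output updates the percentage readout and the minigame's rods.
; On entering the minigame, the slider starts at the target pressure from the minigame data.
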(event `self.MinigameListener.OnEnterMinigame`
  (params (Minigame :type "Minigame Object Reference"))
  (bind _asbp_reactor_minigame (cast `/Game/Blueprints/Minigames/BP_ReactorMinigame` Minigame))
  (bind _output_get (set `self.ReactorMinigame` _asbp_reactor_minigame))
  (`ReactorSliderComponent.SetPercent` (`self.ControlRodSlider`) (`/Game/Blueprints/Minigames/BP_ReactorDataAsset.TargetPressure` (`/Game/Blueprints/Minigames/BP_ReactorMinigame.MinigameData` _output_get))))

(event `self.InteractionComponent.OnInteract`
  (params (OtherPawn :type "Pawn Object Reference") (OtherController :type "PlayerController Object Reference"))
  (`PlayerController.SetViewTargetWithBlend` OtherController (`self.ViewCamera`) (`self.CameraDelay`) "VTBlend_Linear" 0.0 false))

(event `self.ControlRodSlider.OnReset`
  (params (InputValue :type "Float (single-precision)") (OutputValue :type "Float (single-precision)"))
  (`self.SetLeverAngle` InputValue)
  (`self.SetRodsMeter` OutputValue))

(event `self.ControlRodSlider.OnInputChanged`
  (params (NewValue :type "Float (single-precision)") (OldValue :type "Float (single-precision)"))
  (`self.SetLeverAngle` NewValue))

(event `self.InteractionComponent.OnLeave`
  (params (OtherPawn :type "Pawn Object Reference") (OtherController :type "PlayerController Object Reference"))
  (`PlayerController.SetViewTargetWithBlend` OtherController OtherPawn (`self.CameraDelay`) "VTBlend_Linear" 0.0 false))

(event `self.ControlRodSlider.OnOutputChanged`
  (params (NewValue :type "Float (single-precision)") (OldValue :type "Float (single-precision)"))
  (bind _reactorminigame (`self.ReactorMinigame`))
  (`self.SetRodsMeter` NewValue)
  (`/Engine/EditorBlueprintResources/StandardMacros.IsValid` _reactorminigame
    (:`Is Valid`
      (`PercentInputBlock.SetPercent` (`/Game/Blueprints/Minigames/BP_ReactorMinigame.Rods` _reactorminigame) NewValue))))

(event `SetLeverAngle`
  (params (NewAngle :type "Float (single-precision)"))
  (bind _maxleverangle (`self.MaxLeverAngle`))
  (`SceneComponent.K2_SetRelativeRotation` (`self.LeverMesh`) (`KismetMathLibrary.MakeRotator` 0.0 (`KismetMathLibrary.Lerp` (* -1.0 _maxleverangle) _maxleverangle NewAngle)) false false))

(event `SetRodsMeter`
  (params (Value :type "Float (single-precision)"))
  (`TextRenderComponent.K2_SetText` (`self.RodsMeterText`) (`|FormatText` "Rods {VAL}" (`KismetTextLibrary.AsPercent_Float` Value "HalfToEven" false true 1 324 0 0))))

(fn `UserConstructionScript`)