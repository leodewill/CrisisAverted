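; BP_SteamGenerator is an interactable reactor station where the player sets the steam level for the reactor minigame, blending to its own camera while in use.
; Entering the minigame seeds SteamSpeedSlider with the starting steam from the minigame data.
; The slider's input value tilts the lever mesh.
; Its separate output value updates the percentage meter text and is pushed into the minigame's Steam value.
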(event `self.MinigameListener.OnEnterMinigame`
  (params (Minigame :type "Minigame Object Reference"))
  (bind _asbp_reactor_minigame (cast `/Game/Blueprints/Minigames/BP_ReactorMinigame` Minigame))
  (bind _output_get (set `self.ReactorMinigame` _asbp_reactor_minigame))
  (`ReactorSliderComponent.SetPercent` (`self.SteamSpeedSlider`) (`/Game/Blueprints/Minigames/BP_ReactorDataAsset.GetStartSteam` (`/Game/Blueprints/Minigames/BP_ReactorMinigame.MinigameData` _output_get))))

(event `self.InteractionComponent.OnInteract`
  (params (OtherPawn :type "Pawn Object Reference") (OtherController :type "PlayerController Object Reference"))
  (`PlayerController.SetViewTargetWithBlend` OtherController (`self.ViewCamera`) (`self.CameraDelay`) "VTBlend_Linear" 0.0 false))

(event `self.SteamSpeedSlider.OnReset`
  (params (InputValue :type "Float (single-precision)") (OutputValue :type "Float (single-precision)"))
  (`self.SetLeverAngle` InputValue)
  (`self.SetSteamMeter` OutputValue))

(event `self.SteamSpeedSlider.OnInputChanged`
  (params (NewValue :type "Float (single-precision)") (OldValue :type "Float (single-precision)"))
  (`self.SetLeverAngle` NewValue))

(event `self.InteractionComponent.OnLeave`
  (params (OtherPawn :type "Pawn Object Reference") (OtherController :type "PlayerController Object Reference"))
  (`PlayerController.SetViewTargetWithBlend` OtherController OtherPawn (`self.CameraDelay`) "VTBlend_Linear" 0.0 false))

(event `self.SteamSpeedSlider.OnOutputChanged`
  (params (NewValue :type "Float (single-precision)") (OldValue :type "Float (single-precision)"))
  (bind _reactorminigame (`self.ReactorMinigame`))
  (`self.SetSteamMeter` NewValue)
  (`/Engine/EditorBlueprintResources/StandardMacros.IsValid` _reactorminigame
    (:`Is Valid`
      (`PercentInputBlock.SetPercent` (`/Game/Blueprints/Minigames/BP_ReactorMinigame.Steam` _reactorminigame) NewValue))))

(event `SetLeverAngle`
  (params (NewAngle :type "Float (single-precision)"))
  (bind _maxleverangle (`self.MaxLeverAngle`))
  (`SceneComponent.K2_SetRelativeRotation` (`self.LeverMesh`) (`KismetMathLibrary.MakeRotator` (`KismetMathLibrary.Lerp` _maxleverangle (* _maxleverangle -1.0) NewAngle)) false false))

(event `SetSteamMeter`
  (params (Value :type "Float (single-precision)"))
  (`TextRenderComponent.K2_SetText` (`self.SteamMeterText`) (`|FormatText` "Steam {VAL}" (`KismetTextLibrary.AsPercent_Float` Value "HalfToEven" false true 1 324 0 0))))

(fn `UserConstructionScript`)