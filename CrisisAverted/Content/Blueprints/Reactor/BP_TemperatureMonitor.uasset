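; Reactor minigame monitor that shows the current temperature against its target as percentages on a text render.
; On entering the minigame it caches the starting target as a baseline and binds to the Temperature block's value, target and status events.
; The readout shifts the value by its offset from the live target, so the displayed target stays at the baseline.
; Status switches the text between good and bad colors.
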(event `self.MinigameListener.OnEnterMinigame`
  (params (Minigame :type "Minigame Object Reference"))
  (bind _asbp_reactor_minigame (cast `/Game/Blueprints/Minigames/BP_ReactorMinigame` Minigame))
  (`|ExecutionSequence`
    (:`then_0`
      (bind _output_get (set `self.BaseTemperature` (`/Game/Blueprints/Minigames/BP_ReactorDataAsset.TargetTemperature` (`/Game/Blueprints/Minigames/BP_ReactorMinigame.MinigameData` _asbp_reactor_minigame))))
      (`self.OnTemperatureChanged` _output_get _output_get)
      (`self.OnStatusChanged` "Good" "Good"))
    (:`then_1`
      (`self.BindTemperatureListeners` (`/Game/Blueprints/Minigames/BP_ReactorMinigame.Temperature` _asbp_reactor_minigame)))))

(event `BindTemperatureListeners`
  (params (TemperatureBlock :type "UnstableOutputBlock Object Reference"))
  (`|ExecutionSequence`
    (:`then_0`
      (add `UnstableOutputBlock.OnValueChanged` TemperatureBlock (delegate `OnTemperatureChanged`)))
    (:`then_1`
      (add `UnstableOutputBlock.OnTargetChanged` TemperatureBlock (delegate `OnTargetTemperatureChanged`)))
    (:`then_2`
      (add `UnstableOutputBlock.OnStatusChanged` TemperatureBlock (delegate `OnStatusChanged`)))))

(event `OnTemperatureChanged`
  (params (Value :type "Float (single-precision)") (TargetValue :type "Float (single-precision)"))
  (bind _output_get (set `self.Temperature` Value))
  (`self.SetTemperatureText` _output_get TargetValue))

(event `SetTemperatureText`
  (params (Value :type "Float (single-precision)") (TargetValue :type "Float (single-precision)"))
  (`TextRenderComponent.K2_SetText` (`self.TemperatureText`) (`|FormatText` "Temperature: {VAL} / {BASE}" (`KismetTextLibrary.AsPercent_Float` (+ (- Value TargetValue) (`self.BaseTemperature`)) "HalfToEven" false true 1 324 0 0) (`KismetTextLibrary.AsPercent_Float` (`self.BaseTemperature`) "HalfToEven" false true 1 324 0 0))))

(event `OnTargetTemperatureChanged`
  (params (Value :type "Float (single-precision)"))
  (`self.SetTemperatureText` (`self.Temperature`) Value))

(event `OnStatusChanged`
  (params (Status :type "EUnstableMinigameStatus Enum" :default "Low") (OldStatus :type "EUnstableMinigameStatus Enum" :default "Low"))
  (bind _badcolor (`self.BadColor`))
  (`TextRenderComponent.SetTextRenderColor` (`self.TemperatureText`) (select `EUnstableMinigameStatus` Status :`Low` _badcolor :`Good` (`self.GoodColor`) :`High` _badcolor)))

(fn `UserConstructionScript`)