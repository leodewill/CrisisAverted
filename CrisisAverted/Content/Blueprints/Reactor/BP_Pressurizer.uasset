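; BP_Pressurizer is an interactable pressurizer station for the reactor minigame that blends the player's view to its own camera while in use.
; On minigame entry it seeds pressure from the target value.
; Open heater and water valves raise or lower pressure over time, updating a percent readout and the minigame's Pressurizer.
; All three valves move their buttons on open and close; the vent valve does not affect pressure here.
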(event `self.MinigameListener.OnEnterMinigame`
  (params (Minigame :type "Minigame Object Reference"))
  (bind _asbp_reactor_minigame (cast `/Game/Blueprints/Minigames/BP_ReactorMinigame` Minigame))
  (bind _output_get (set `self.ReactorMinigame` _asbp_reactor_minigame))
  (set `self.Pressure` (`/Game/Blueprints/Minigames/BP_ReactorDataAsset.TargetPressure` (`/Game/Blueprints/Minigames/BP_ReactorMinigame.MinigameData` _output_get))))

(event `self.HeaterValve.OnGape`
  (params (Speed :type "Float (single-precision)") (DeltaSeconds :type "Float (single-precision)"))
  (`self.OnPressureChanged` (+ (`self.Pressure`) (* Speed DeltaSeconds))))

(event `OnPressureChanged`
  (params (InPressure :type "Float (double-precision)"))
  (bind _output_get (set `self.Pressure` (`KismetMathLibrary.FClamp` InPressure)))
  (`self.SetPressureMeter` _output_get)
  (`self.Process`))

(event `self.WaterValve.OnGape`
  (params (Speed :type "Float (single-precision)") (DeltaSeconds :type "Float (single-precision)"))
  (`self.OnPressureChanged` (- (`self.Pressure`) (* Speed DeltaSeconds))))

(event `Process`
  (`PercentInputBlock.SetPercent` (`/Game/Blueprints/Minigames/BP_ReactorMinigame.Pressurizer` (`self.ReactorMinigame`)) (`self.Pressure`)))

(event `self.InteractionComponent.OnInteract`
  (params (OtherPawn :type "Pawn Object Reference") (OtherController :type "PlayerController Object Reference"))
  (`PlayerController.SetViewTargetWithBlend` OtherController (`self.ViewCamera`) (`self.CameraDelay`) "VTBlend_Linear" 0.0 false))

(event `self.HeaterValve.OnOpen`
  (`self.SetButtonState` (`self.HeaterButton`) true))

(event `SetPressureMeter`
  (params (Value :type "Float (single-precision)"))
  ;[1 1 1] Visuals
  (`TextRenderComponent.K2_SetText` (`self.PressureMeterText`) (`|FormatText` "Pressure {VAL}" (`KismetTextLibrary.AsPercent_Float` Value "HalfToEven" false true 1 324 0 0))))

(event `self.HeaterValve.OnClose`
  (`self.SetButtonState` (`self.HeaterButton`)))

(event `SetButtonState`
  (params (Button :type "SceneComponent Object Reference") (bPressed :type Boolean))
  (bind (_relativelocation_x _relativelocation_y) (`KismetMathLibrary.BreakVector` (`SceneComponent.RelativeLocation` Button)))
  ;[1 1 1] Visuals
  (`SceneComponent.K2_SetRelativeLocation` Button (`KismetMathLibrary.MakeVector` _relativelocation_x _relativelocation_y (`KismetMathLibrary.SelectFloat` (`self.PressedButtonHeight`) (`self.UnpressetButtonHeight`) bPressed)) false false))

(event `self.InteractionComponent.OnLeave`
  (params (OtherPawn :type "Pawn Object Reference") (OtherController :type "PlayerController Object Reference"))
  (`PlayerController.SetViewTargetWithBlend` OtherController OtherPawn (`self.CameraDelay`) "VTBlend_Linear" 0.0 false))

(event `self.WaterValve.OnOpen`
  (`self.SetButtonState` (`self.WaterButton`) true))

(event `self.WaterValve.OnClose`
  (`self.SetButtonState` (`self.WaterButton`)))

(event `self.VentValve.OnOpen`
  (`self.SetButtonState` (`self.VentButton`) true))

(event `self.VentValve.OnClose`
  (`self.SetButtonState` (`self.VentButton`)))

(fn `UserConstructionScript`)