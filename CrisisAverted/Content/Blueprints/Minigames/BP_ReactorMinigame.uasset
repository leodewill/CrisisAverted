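; BP_ReactorMinigame is a reactor minigame Blueprint that links a Steam value to a Power value.
; Whenever Steam changes, the Process event copies its percentage straight into Power.
; Start, expiry and Power changes only print debug messages, showing the starting Steam, a ding, or the Power percentage and status.
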(event `self.OnStart`
  (`KismetSystemLibrary.PrintString` (`KismetTextLibrary.Conv_TextToString` (`|FormatText` "STARTING WITH {VAL} Steam" (`KismetTextLibrary.AsPercent_Float` (`PercentInputBlock.GetPercent` (`self.Steam`)) "HalfToEven")))))

(event `self.OnExpired`
  (`KismetSystemLibrary.PrintString` "DING DING"))

(event `self.Power.OnChanged`
  (params (Value :type "Float (single-precision)") (Status :type "EUnstableMinigameStatus Enum" :default "Low"))
  (`KismetSystemLibrary.PrintString` (`KismetTextLibrary.Conv_TextToString` (`|FormatText` "Power {VAL} ({STAT}" (`KismetTextLibrary.AsPercent_Float` Value "HalfToEven") (`|GetEnumeratorName` Status)))))

(event `self.Steam.OnChanged`
  (params (Value :type "Float (single-precision)"))
  (`self.Process`))

(event `Process`
  (`UnstableOutputBlock.SetPercent` (`self.Power`) (`PercentInputBlock.GetPercent` (`self.Steam`))))

(fn `UserConstructionScript`)