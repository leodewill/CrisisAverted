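; Reactor minigame data asset that holds tuning values and the formulas for steam, demand and pressure.
; Starting steam equals the start demand.
; Each next demand moves by a random variation toward the opposite half of its range, down from 0.5 or above and up otherwise, clamped to 0–1.
; Pressure is the pressurizer value plus steam's deviation from its start, scaled by a multiplier.
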(fn `GetNextDemand`
  (params (Demand :type "Float (double-precision)"))
  (returns (NextDemand :type "Float (double-precision)"))
  (locals (Direction :type Integer) (Variation :type "Float (double-precision)" :default 0.0))
  (return (`KismetMathLibrary.FClamp` (+ Demand (* (`KismetMathLibrary.SelectFloat` -1.0 1.0 (>= Demand 0.5)) (`KismetMathLibrary.RandomFloatInRange` (`self.MinDemandVariation`) (`self.MaxDemandVariation`)))))))

(fn `GetPressure`
  (params (Pressurizer :type "Float (double-precision)") (Steam :type "Float (double-precision)"))
  (returns (Pressure :type "Float (double-precision)"))
  (return (+ Pressurizer (* (- Steam (`self.GetStartSteam`)) (`self.SteamPressureMultiplier`)))))

(fn `GetStartSteam`
  (returns (Value :type "Float (double-precision)"))
  (return (`self.StartDemand`)))