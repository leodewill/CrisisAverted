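; DialogueManager is an actor that owns the on-screen dialogue widget and controls its display.
; On BeginPlay it creates a DialogueWidget for player 0, adds it to the viewport and hides it.
; Its SetVisibility and SetWidgetText events pass visibility and text changes through to that widget, with no dialogue logic of its own.
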(event `self.ReceiveBeginPlay`
  (bind _returnvalue (`|CreateWidget` "/Game/Blueprints/DialogueSystem/DialogueWidget.DialogueWidget_C" (`GameplayStatics.GetPlayerController` 0)))
  (bind _output_get (set `self.Widget` _returnvalue))
  (`UserWidget.AddToViewport` _output_get 0)
  (`Widget.SetVisibility` _output_get "Hidden"))

(event `SetVisibility`
  (params (InVisibility :type "ESlateVisibility Enum" :default "Visible"))
  (`Widget.SetVisibility` (`self.Widget`) InVisibility))

(event `SetWidgetText`
  (params (CurrentTextVar :type Text))
  (`/Game/Blueprints/DialogueSystem/DialogueWidget.SetNewText` (`self.Widget`) CurrentTextVar))

(fn `UserConstructionScript`)